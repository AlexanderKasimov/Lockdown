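; GM_Gameplay is the gameplay game mode that sets up a session, starts play and tracks hit points until the game is lost.
; BeginPlay finds the Player pawn and EnemySpawner actors, hands the pawn to PlayerController_Gameplay, and creates the main widget to play its intro.
; StartGame forwards to the controller, while FinishStartingGame shows the gameplay UI and activates every spawner.
; ReceiveDamage reduces HP and, at zero, flags the game ended once with only a printed loss message.
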(event Custom|ReceiveDamage
  (params (Damage :type Float%20%28single-precision%29))
  (Variables|Default|SetCurHP (- (Variables|Default|GetCurHP) Damage))
  (if (and (<= (Variables|Default|GetCurHP) 0.0) (not (Variables|Default|GetisGameEnded)))
    (Variables|Default|SetisGameEnded true)
    (Development|PrintString "LOST!!!!")))

(event Custom|StartGame
  (Default|StartGame (Variables|Default|GetPlayerController)))

(event Custom|FinishStartingGame
  (Utilities|FlowControl|Sequence
    (:then_0
      (Default|ShowGameplay (Variables|Default|GetUI_MainWidget)))
    (:then_1
      (for _array_element (Variables|Default|GetSpawners)
        (Default|Activate _array_element)))))

(event EventBeginPlay
  (Utilities|FlowControl|Sequence
    (:then_0
      (bind _outactors (Actor|GetAllActorsOfClass "/Game/BP/Player/Player.Player_C"))
      (Variables|Default|SetPlayerPawn (Utilities|Array|Get(acopy) _outactors)))
    (:then_1
      (bind _returnvalue (UserInterface|CreateWidget "/Game/UI/UI_MainWidget.UI_MainWidget_C"))
      (bind _output_get (Variables|Default|SetUI_MainWidget _returnvalue))
      (UserInterface|Viewport|AddtoViewport _output_get 0))
    (:then_2
      (bind _asplayer_controller_gameplay (Utilities|Casting|CastToPlayerController_Gameplay (Game|GetPlayerController 0)))
      (Variables|Default|SetPlayerController _asplayer_controller_gameplay)
      (Variables|/Game/BP/Player/PlayerController_Gameplay.PlayerController_Gameplay_C|SetPlayerPawn (Variables|Default|GetPlayerController) (Variables|Default|GetPlayerPawn)))
    (:then_3
      (Default|PlayIntro (Variables|Default|GetUI_MainWidget)))
    (:then_4
      (bind _outactors_2 (Actor|GetAllActorsOfClass "/Game/BP/EnemySpawner.EnemySpawner_C"))
      (Variables|Default|SetSpawners _outactors_2))
    (:then_5
      (Variables|Default|SetCurHP (Variables|Default|GetHP)))))

(event EventTick
  (params (DeltaSeconds :type Float%20%28single-precision%29)))

(fn ConstructionScript)