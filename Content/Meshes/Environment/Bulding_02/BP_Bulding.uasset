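; BP_Bulding is a modular building actor assembled from base, story and top meshes, with an adjustable story count.
; The construction script sets the base mesh, then adds story mesh components in a loop from zero through StoryNumber, stacked upward using mesh bounds heights.
; Each story is stored in an array, and the top mesh sits one story height above the last entry.
; The event graph has no logic.
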(event EventBeginPlay)

(event Collision|EventActorBeginOverlap
  (params (OtherActor :type Actor%20Object%20Reference)))

(event EventTick
  (params (DeltaSeconds :type Float%20%28single-precision%29)))

(fn ConstructionScript
  (bind _storymesh (Variables|Default|GetStoryMesh))
  (bind _storysarray (Variables|Default|GetStorysArray))
  (Components|StaticMesh|SetStaticMesh (Variables|Default|GetStaticMesh) (Variables|Default|GetBaseMesh))
  (for _index (range 0 (Variables|Default|GetStoryNumber))
    (bind _returnvalue (AddComponent|AddStaticMeshComponent false (Math|Transform|MakeTransform (+ (Math|Vector|MakeVector 0.0 0.0 (* 2 (.Z (Math|Vector|BreakVector (.BoxExtent (Collision|GetComponentBounds (Variables|Default|GetStaticMesh))))))) (* (Math|Vector|MakeVector 0.0 0.0 (.Z (Math|Vector|BreakVector (* (.boxextent (StaticMesh|GetBounds _storymesh)) 2)))) _index)) "0, 0, 0" "1,1,1")))
    (Utilities|Array|Add (Variables|Default|GetStorysArray) _returnvalue)
    (Components|StaticMesh|SetStaticMesh _returnvalue _storymesh))
  (bind _returnvalue_2 (AddComponent|AddStaticMeshComponent false (Math|Transform|MakeTransform (+ (Math|Vector|MakeVector 0.0 0.0 (.Z (Math|Vector|BreakVector (* (.boxextent (StaticMesh|GetBounds (Variables|Default|GetStoryMesh))) 2)))) (Variables|/Script/Engine.SceneComponent|GetRelativeLocation (Utilities|Array|Get(acopy) _storysarray (- (Utilities|Array|Length _storysarray) 1)))) "0, 0, 0" "1,1,1")))
  (Components|StaticMesh|SetStaticMesh _returnvalue_2 (Variables|Default|GetTopMesh)))